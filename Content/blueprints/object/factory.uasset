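; Factory actor that displays a Paper2D sprite, levels up when clicked and earns money for the player.
; Tick refreshes the sprite and, through a DoOnce gated by an externally set click flag, raises the level and advances through a sprite array until its last entry.
; A one-second Delay on Tick throttles income, adding the square of level times a money multiplier to the pawn_game total.
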(event `self.ReceiveTick`
  (params (DeltaSeconds :type "Float (single-precision)"))
  (`|ExecutionSequence`
    (:`then_0`
      (`PaperSpriteComponent.SetSprite` (`self.PaperSprite`) (`self.defoult_sprite`)))
    (:`then_1`
      (if (`self.on cliced`)
        (`/Engine/EditorBlueprintResources/StandardMacros.DoOnce` false :!label _label
          (:`Completed`
            (if (> (`KismetArrayLibrary.Array_LastIndex` (`self.array_off_factory_sprites`)) (`self.defoult_number_of_factorry`))
              (`/Engine/EditorBlueprintResources/StandardMacros.IncrementInt` (`self.level_factory`)
                (:`  `
                  (bind _result (`/Engine/EditorBlueprintResources/StandardMacros.IncrementInt` (`self.defoult_number_of_factorry`))
                    (:`  `
                      (set `self.defoult_sprite` (`|GetArrayItem` (`self.array_off_factory_sprites`) _result))
                      (set `self.on cliced` false))))))))
        (else
          (goto _label :!via `Reset`))))
    (:`then_2`
      (`KismetSystemLibrary.Delay` 1.0)
      (bind _aspawn_game (cast `/Game/blueprints/pawn/pawn_game` (`GameplayStatics.GetPlayerPawn` 0)))
      (set `/Game/blueprints/pawn/pawn_game.all_money` (+ (`/Game/blueprints/pawn/pawn_game.all_money` _aspawn_game) (`KismetMathLibrary.Square` (* (`self.level_factory`) (`self.defoult_money_up`)))) _aspawn_game))))

(fn `UserConstructionScript`)