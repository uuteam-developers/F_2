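; Factory worker actor that walks to the location of a referenced ActorToMove while its IsCliced flag is set.
; Each Tick picks directions and steps one unit by local offset, aligning X before moving along Y, with no delta-time scaling or sweep.
; It clears the flag on arrival and refreshes the cached target location after the movement step.
; An unconnected check against main's EnableActor does nothing.
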(event `self.ReceiveTick`
  (params (DeltaSeconds :type "Float (single-precision)"))
  (bind _x (.x (`self.K2_GetActorLocation`)))
  (bind _y (.y (`self.K2_GetActorLocation`)))
  (bind _x_2 (.x (`self.get location to go`)))
  (bind _y_2 (.y (`self.get location to go`)))
  (bind _returnvalue (`KismetMathLibrary.NearlyEqual_FloatFloat` _x _x_2 1.0))
  (`|ExecutionSequence`
    (:`then_0`
      (if (`self.is cliced`)
        (`|ExecutionSequence`
          (:`then_0`
            (`|ExecutionSequence`
              (:`then_0`
                (if (and _returnvalue (`KismetMathLibrary.NearlyEqual_FloatFloat` _y _y_2 1.0))
                  (set `self.is cliced` false)
                  (set `self.move_y` false)
                  (set `self.move` false)
                  (else
                    (set `self.move` true))))
              (:`then_1`
                (if _returnvalue
                  (set `self.move_y` true)
                  (elif (< _x _x_2)
                    (set `self.go up` true)
                    (else
                      (set `self.go up` false)))))
              (:`then_2`
                (if (`KismetMathLibrary.NearlyEqual_FloatFloat` _y _y_2 10.0)
                  _
                  (elif (< _y _y_2)
                    (set `self.go left` false)
                    (else
                      (set `self.go left` true)))))))
          (:`then_1`
            (if (`self.move`)
              (if (`self.move_y`)
                (if (`self.go left`)
                  (`self.K2_AddActorLocalOffset` (0.0 -1.0 0.0))
                  (else
                    (`self.K2_AddActorLocalOffset` (0.0 1.0 0.0))))
                (elif (`self.go up`)
                  (`self.K2_AddActorLocalOffset` (1.0 0.0 0.0))
                  (else
                    (`self.K2_AddActorLocalOffset` (-1.0 0.0 0.0))))))))))
    (:`then_1`
      (set `self.get location to go` (`self.K2_GetActorLocation` (`self.actor to move`))))))

(fn `UserConstructionScript`)