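; A zombie enemy that picks a random Controll_point on spawn, gets a random sprite and walks toward that point.
; Each tick it yaws its arrow at the target and steps along it by a fixed amount until closer than Speed.
; It also calls a damage macro, shown empty here, and copies HitPoint to its widget.
; At zero health it adds one money to the player pawn and destroys itself.
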(event `self.ReceiveBeginPlay`
  (`|ExecutionSequence`
    (:`then_0`
      (bind _output (`self.set target`)
        (:`out`
          (set `self.attac_target` _output)
          (`PaperSpriteComponent.SetSprite` (`self.PaperSprite`) (`|GetArrayItem` (`self.array`) (`KismetMathLibrary.RandomIntegerInRange` 0 2))))))))

(event `self.ReceiveTick`
  (params (DeltaSeconds :type "Float (single-precision)"))
  (`/Engine/EditorBlueprintResources/StandardMacros.IsValid` (`self.attac_target`)
    (:`Is Valid`
      (`|ExecutionSequence`
        (:`then_0`
          (`self.set rotation(look at target)`))
        (:`then_1`
          (`self.set velosity`))
        (:`then_2`
          (`self.give_damage` (`self.is damage`) (`self.damage`)))
        (:`then_3`
          (bind _ashit_point (cast `/Game/wiget/hit_point` (`WidgetComponent.GetUserWidgetObject` (`self.Widget`))))
          (set `/Game/wiget/hit_point.hit_point` (`self.hit_point`) _ashit_point))
        (:`then_4`
          (if (<= (`self.hit_point`) 0.0)
            (bind _aspawn_game (cast `/Game/blueprints/pawn/pawn_game` (`GameplayStatics.GetPlayerPawn` 0)))
            (set `/Game/blueprints/pawn/pawn_game.all_money` (+ (`/Game/blueprints/pawn/pawn_game.all_money` _aspawn_game) 1.0) _aspawn_game)
            (`self.K2_DestroyActor`)))))))

(fn `UserConstructionScript`)