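; Turret actor that scans for zombies and shoots at them, driven by an IsChill idle/attack switch on Tick.
; While idle it sweeps its Scene component back and forth while a short debug-drawn line trace looks for "zb"-tagged actors.
; With a target it yaws to face it, spawning a Bullet and cosmetic Bullet_trash after each delay.
; Dmage also subtracts zombie HitPoint directly, and an invalid target returns it to idle.
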(event `self.ReceiveTick`
  (params (DeltaSeconds :type "Float (single-precision)"))
  (`|ExecutionSequence`
    (:`then_0`
      (if (`self.is chill`)
        (`|ExecutionSequence`
          (:`then_0`
            (`self.rotate_look`))
          (:`then_1`
            (`self.find target`)))
        (else
          (`/Engine/EditorBlueprintResources/StandardMacros.IsValid` (`self.target focus`)
            (:`Is Valid`
              (`|ExecutionSequence`
                (:`then_0`
                  (if (`self.is attack`)
                    (`KismetSystemLibrary.Delay` (`self.speed_shoot`))
                    (bind _returnvalue (`|SpawnActorFromClass` "/Game/blueprints/object/bullet.bullet_C" (`KismetMathLibrary.Conv_VectorToTransform` (`SceneComponent.K2_GetComponentLocation` (`self.Arrow`))) "Undefined" "OverrideRootScale" null null))
                    (set `/Game/blueprints/object/bullet.forward vector` (`self.forward vector`) _returnvalue)
                    (set `/Game/blueprints/object/bullet.attac target` (`self.target focus`) _returnvalue)
                    (set `/Game/blueprints/object/bullet.damage` (`self.damage`) _returnvalue)
                    (set `self.is attack` false)
                    (`self.Dmage`)))
                (:`then_1`
                  (`/Engine/EditorBlueprintResources/StandardMacros.IsValid` (`self.target focus`)
                    (:`Is Valid`
                      (`self.rotate to look at target`))
                    (:`Is Not Valid`
                      (set `self.is chill` true))))))
            (:`Is Not Valid`
              (set `self.is chill` true))))))))

(fn `UserConstructionScript`)