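; Bullet actor that flies toward a target and damages zombies on contact.
; Each tick it teleports-free steps along a stored ForwardVector by Speed, and destroys itself once its AttacTarget is no longer valid.
; When its Sphere overlaps an actor tagged "zb", it sets the zombie's damage flag and amount directly, then destroys itself.
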(event `self.ReceiveTick`
  (params (DeltaSeconds :type "Float (single-precision)"))
  (`/Engine/EditorBlueprintResources/StandardMacros.IsValid` (`self.attac target`)
    (:`Is Valid`
      (`|ExecutionSequence`
        (:`then_1`
          (`self.K2_SetActorLocation` (+ (`self.K2_GetActorLocation`) (* (`self.forward vector`) (`self.speed`)))))))
    (:`Is Not Valid`
      (`self.K2_DestroyActor`))))

(event `self.Sphere.OnComponentBeginOverlap`
  (params (OverlappedComponent :type "PrimitiveComponent Object Reference") (OtherActor :type "Actor Object Reference") (OtherComp :type "PrimitiveComponent Object Reference") (OtherBodyIndex :type Integer) (bFromSweep :type Boolean) (SweepResult :type "HitResult Structure (by ref)"))
  (if (`self.ActorHasTag` OtherActor "zb")
    (bind _aszombie (cast `/Game/blueprints/object/zombie` OtherActor))
    (set `/Game/blueprints/object/zombie.is damage` true _aszombie)
    (set `/Game/blueprints/object/zombie.damage` (`self.damage`) _aszombie)
    (`self.K2_DestroyActor`)))

(fn `UserConstructionScript`)