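; Player pawn for a click-driven game with money, factories and turrets, handling mouse interaction and the money display.
; It shows the cursor at start and writes AllMoney to the Number text every tick.
; On left click it traces under the cursor on Visibility, then uses actor tags and casts to set OnCliced on the hit factory, factory spawner or turret spawner.
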(event `self.ReceiveTick`
  (params (DeltaSeconds :type "Float (single-precision)"))
  (`TextRenderComponent.K2_SetText` (`self.number`) (`KismetTextLibrary.Conv_DoubleToText` (`self.all_money`) "HalfToEven")))

(event `self.ReceiveBeginPlay`
  (set `PlayerController.bShowMouseCursor` true (`GameplayStatics.GetPlayerController` 0)))

(event `Key|LeftMouseButton`
  (params (Key :type "Key Structure"))
  (bind (_hitresult _returnvalue) (`PlayerController.GetHitResultUnderCursorByChannel` (`GameplayStatics.GetPlayerController` 0) "TraceTypeQuery1" true))
  (bind (_bblockinghit _binitialoverlap _time _distance _location _impactpoint _normal _impactnormal _physmat _hitactor) (`GameplayStatics.BreakHitResult` _hitresult))
  (:`Pressed`
    (if _returnvalue
      (`|ExecutionSequence`
        (:`then_0`
          (if (`self.ActorHasTag` _hitactor "factory")
            (bind _asfactory (cast `/Game/blueprints/object/factory` _hitactor))
            (set `/Game/blueprints/object/factory.on cliced` true _asfactory)))
        (:`then_1`
          (if (`self.ActorHasTag` _hitactor "spf")
            (bind _asspawner_factory (cast `/Game/blueprints/spawner/spawner_factory` _hitactor))
            (set `/Game/blueprints/spawner/spawner_factory.on cliced` true _asspawner_factory)))
        (:`then_2`
          (if (`self.ActorHasTag` _hitactor "spt")
            (bind _asturret_spawner (cast `/Game/blueprints/spawner/turret_spawner` _hitactor))
            (set `/Game/blueprints/spawner/turret_spawner.on_cliced` true _asturret_spawner)))))))

(fn `UserConstructionScript`)