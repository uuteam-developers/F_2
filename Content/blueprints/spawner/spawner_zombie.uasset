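; Spawner actor that continuously spawns Zombie actors at one of three marker points.
; BeginPlay caches the world locations of its three scene components in an array.
; Tick feeds a Delay node, whose ignoring of re-triggers while pending turns it into a repeating timer set by a Delay variable.
; Each completed delay spawns a Zombie at a randomly picked cached location, with no count limit.
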(event `self.ReceiveBeginPlay`
  (`KismetArrayLibrary.Array_Add` (`self.array_of_location`) (`SceneComponent.K2_GetComponentLocation` (`self.Scene3`)))
  (`KismetArrayLibrary.Array_Add` (`self.array_of_location`) (`SceneComponent.K2_GetComponentLocation` (`self.Scene2`)))
  (`KismetArrayLibrary.Array_Add` (`self.array_of_location`) (`SceneComponent.K2_GetComponentLocation` (`self.Scene1`))))

(event `self.ReceiveTick`
  (params (DeltaSeconds :type "Float (single-precision)"))
  (`|ExecutionSequence`
    (:`then_0`
      (`KismetSystemLibrary.Delay` (`self.delay`))
      (`|SpawnActorFromClass` "/Game/blueprints/object/zombie.zombie_C" (`KismetMathLibrary.Conv_VectorToTransform` (`|GetArrayItem` (`self.array_of_location`) (`KismetMathLibrary.RandomIntegerInRange` 0 2))) "Undefined" "OverrideRootScale" null null))))

(fn `UserConstructionScript`)